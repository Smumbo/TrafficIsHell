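; DemonAI is an enemy character that moves toward the FirstPersonCharacterTentacles player when seen, and is destroyed when IncomingDamage drains its Health.
; It also carries a modular trooper preset demo: E or gamepad face button left cycles six male, female and plain-form looks.
; Each preset swaps meshes, anim classes and materials on head, armor, helmet and hair components.
; The construction script slaves upper, lower and shoulder meshes to the main Mesh via master pose.
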(event `self.PawnSensing.OnSeePawn`
  (params (Pawn :type "Pawn Object Reference"))
  (if (`KismetSystemLibrary.IsValid` Pawn)
    (bind _asfirst_person_character_tentacles (cast `/Game/FirstPersonBP/Blueprints/FirstPersonCharacterTentacles` Pawn))
    (`|AIMoveTo` self (0.0 0.0 0.0) _asfirst_person_character_tentacles 10.0)))

(event `self.ReceiveBeginPlay`
  (`|ExecutionSequence`
    (:`then_0`
      ;[1 1 1] Hiding body sections
      (for _index (range 5 15)
        (`SkinnedMeshComponent.ShowMaterialSection` (`self.Mesh`) _index 0 false 0)))
    (:`then_1`
      ;[1 1 1] Initializing CharIndex
      (bind _output_get (set `self.CharPresetIndex` 0))
      (`KismetSystemLibrary.PrintString` (`KismetStringLibrary.Conv_IntToString` _output_get))
      (`KismetSystemLibrary.PrintString` "CharBP index is")
      (`KismetSystemLibrary.PrintString` "PRESS E TO CYCLE THROUGH CHARACTER PRESETS" true true (struct :`R` 1.0 :`G` 1.0 :`B` 1.0 :`A` 1.0) 5.0))))

(event `Key|Gamepad_FaceButton_Left`
  (params (Key :type "Key Structure"))
  (bind _mesh (`self.Mesh`))
  (bind _mesh_2 (`self.Mesh`))
  (bind _lower__skeketal_ (`self.Lower (skeketal)`))
  (bind _mesh_3 (`self.Mesh`))
  (bind _mesh_4 (`self.Mesh`))
  (bind _upper__skeletal_ (`self.Upper (skeletal)`))
  (bind _lower__skeketal__2 (`self.Lower (skeketal)`))
  (bind _mesh_5 (`self.Mesh`))
  (bind _lower__skeketal__3 (`self.Lower (skeketal)`))
  (bind _hair_a__socketed_ (`self.Hair_A (socketed)`))
  (bind _helmet__socketed_ (`self.Helmet (socketed)`))
  (bind _mesh_6 (`self.Mesh`))
  (bind _hair_c__socketed_ (`self.Hair_C (socketed)`))
  (bind _upper__skeletal__2 (`self.Upper (skeletal)`))
  (bind _mesh_7 (`self.Mesh`))
  (bind _upper__skeletal__3 (`self.Upper (skeletal)`))
  (bind _hair_a__socketed__2 (`self.Hair_A (socketed)`))
  (bind _shoulders__skeletal_ (`self.Shoulders (skeletal)`))
  (bind _hair_b__socketed_ (`self.Hair_B (socketed)`))
  (bind _upper__skeletal__4 (`self.Upper (skeletal)`))
  (bind _upper__skeletal__5 (`self.Upper (skeletal)`))
  (bind _hair_b__socketed__2 (`self.Hair_B (socketed)`))
  (bind _helmet__socketed__2 (`self.Helmet (socketed)`))
  (bind _helmet__socketed__3 (`self.Helmet (socketed)`))
  (bind _lower__skeketal__4 (`self.Lower (skeketal)`))
  (bind _hair_c__socketed__2 (`self.Hair_C (socketed)`))
  (bind _mesh_8 (`self.Mesh`))
  (bind _helmet__socketed__4 (`self.Helmet (socketed)`))
  (bind _hair_c__socketed__3 (`self.Hair_C (socketed)`))
  (bind _upper__skeletal__6 (`self.Upper (skeletal)`))
  (bind _shoulders__skeletal__2 (`self.Shoulders (skeletal)`))
  (bind _shoulders__skeletal__3 (`self.Shoulders (skeletal)`))
  (bind _shoulders__skeletal__4 (`self.Shoulders (skeletal)`))
  (bind _hair_c__socketed__4 (`self.Hair_C (socketed)`))
  (bind _hair_a__socketed__3 (`self.Hair_A (socketed)`))
  (bind _hair_b__socketed__3 (`self.Hair_B (socketed)`))
  (bind _hair_a__socketed__4 (`self.Hair_A (socketed)`))
  (bind _hair_b__socketed__4 (`self.Hair_B (socketed)`))
  (bind _lower__skeketal__5 (`self.Lower (skeketal)`))
  (bind _mesh_9 (`self.Mesh`))
  (bind _helmet__socketed__5 (`self.Helmet (socketed)`))
  (bind _hair_a__socketed__5 (`self.Hair_A (socketed)`))
  (bind _shoulders__skeletal__5 (`self.Shoulders (skeletal)`))
  (bind _hair_b__socketed__5 (`self.Hair_B (socketed)`))
  (bind _hair_c__socketed__5 (`self.Hair_C (socketed)`))
  (bind _mesh_10 (`self.Mesh`))
  (bind _upper__skeletal__7 (`self.Upper (skeletal)`))
  (bind _lower__skeketal__6 (`self.Lower (skeketal)`))
  (bind _helmet__socketed__6 (`self.Helmet (socketed)`))
  (bind _hair_a__socketed__6 (`self.Hair_A (socketed)`))
  (bind _shoulders__skeletal__6 (`self.Shoulders (skeletal)`))
  (bind _hair_b__socketed__6 (`self.Hair_B (socketed)`))
  (bind _hair_c__socketed__6 (`self.Hair_C (socketed)`))
  (:`Pressed`
    (`|ExecutionSequence` :!label _label
      (:`then_0`
        ;[1 1 1] Cycling character index
        (if (>= (`self.CharPresetIndex`) 5)
          (bind _output_get (set `self.CharPresetIndex` 0))
          (`KismetSystemLibrary.PrintString` (`KismetStringLibrary.Conv_IntToString` _output_get))
          (`KismetSystemLibrary.PrintString` "CharPresetIndex")
          (else
            (bind _output_get_2 (set `self.CharPresetIndex` (+ (`self.CharPresetIndex`) 1)))
            (`KismetSystemLibrary.PrintString` (`KismetStringLibrary.Conv_IntToString` _output_get_2))
            (`KismetSystemLibrary.PrintString` "CharPresetIndex"))))
      (:`then_1`
        ;[1 1 1] Assigning presets to indexes
        (if (== (`self.CharPresetIndex`) 0)
          ;[0.02924 0.4632 1] Set main Mesh component (full body or standalone head)
          (`SkeletalMeshComponent.SetAnimInstanceClass` _mesh_2 "/Game/Action_Trooper/Animations/Male/ThirdPerson_Male_AnimBP.ThirdPerson_Male_AnimBP_C")
          (`SkinnedMeshComponent.SetSkinnedAssetAndUpdate` _mesh_2 "/Game/Action_Trooper/Meshes/Trooper_Heads/SK_M_Trooper_Head_A_White2.SK_M_Trooper_Head_A_White2" false)
          ;[0.02745 0.4627 1] Set material(s) of body or head per ID
          (`|ExecutionSequence`
            (:`then_0`
              (for _index (range 2)
                (`PrimitiveComponent.SetMaterial` _mesh_8 _index "/Game/Action_Trooper/Materials/Trooper_Heads_and_Bodies/MI_Trooper_M_Head_A_White.MI_Trooper_M_Head_A_White")
                ;[0.02745 0.4627 1] Set Upper armor and material
                (`SkeletalMeshComponent.SetAnimInstanceClass` _upper__skeletal__6 "/Game/Action_Trooper/Animations/Male/ThirdPerson_Male_AnimBP.ThirdPerson_Male_AnimBP_C")
                (`SkinnedMeshComponent.SetSkinnedAssetAndUpdate` _upper__skeletal__6 "/Game/Action_Trooper/Meshes/Trooper_Armor_Modular/SK_M_Trooper_Upper.SK_M_Trooper_Upper" false)
                (`PrimitiveComponent.SetMaterial` (`self.Upper (skeletal)`) 0 "/Game/Action_Trooper/Materials/Trooper_Armor/MI_Trooper_Upper_NoTint_Milit.MI_Trooper_Upper_NoTint_Milit")
                ;[0.02924 0.4632 1] Set Lower armor and material
                (`SkeletalMeshComponent.SetAnimInstanceClass` _lower__skeketal__4 "/Game/Action_Trooper/Animations/Male/ThirdPerson_Male_AnimBP.ThirdPerson_Male_AnimBP_C")
                (`SkinnedMeshComponent.SetSkinnedAssetAndUpdate` _lower__skeketal__4 "/Game/Action_Trooper/Meshes/Trooper_Armor_Modular/SK_M_Trooper_Lower.SK_M_Trooper_Lower" false)
                (`PrimitiveComponent.SetMaterial` (`self.Lower (skeketal)`) 0 "/Game/Action_Trooper/Materials/Trooper_Armor/MI_Trooper_NoTint_Lower_Milit.MI_Trooper_NoTint_Lower_Milit")
                ;[0.02745 0.4627 1] Set Shoulders and materials (left/right)
                (`SkeletalMeshComponent.SetAnimInstanceClass` _shoulders__skeletal__4 "/Game/Action_Trooper/Animations/Male/ThirdPerson_Male_AnimBP.ThirdPerson_Male_AnimBP_C")
                (`SkinnedMeshComponent.SetSkinnedAssetAndUpdate` _shoulders__skeletal__4 "/Game/Action_Trooper/Meshes/Trooper_Armor_Modular/SK_M_Trooper_Shoulders_A.SK_M_Trooper_Shoulders_A" false)
                (`|ExecutionSequence`
                  (:`then_0`
                    (`PrimitiveComponent.SetMaterial` _shoulders__skeletal__4 0 "/Game/Action_Trooper/Materials/Trooper_Armor/MI_Trooper_GloFX_Shoulders_Blueglo.MI_Trooper_GloFX_Shoulders_Blueglo")
                    ;[0.02924 0.4632 1] Set Helmet (socketed)
                    (`SkinnedMeshComponent.SetSkinnedAssetAndUpdate` _helmet__socketed__4 "/Game/Action_Trooper/Meshes/Trooper_Helmets/SK_M_Trooper_Helmet_B.SK_M_Trooper_Helmet_B" true)
                    (`|ExecutionSequence`
                      (:`then_0`
                        (`PrimitiveComponent.SetMaterial` _helmet__socketed__4 2 "/Game/Action_Trooper/Materials/Trooper_Armor/MI_Trooper_Helmet_NoTint_Milit.MI_Trooper_Helmet_NoTint_Milit")
                        ;[0.02924 0.4632 1] Set hair and beard (socketed)
                        (`SkinnedMeshComponent.SetSkinnedAssetAndUpdate` _hair_a__socketed_ "/Game/Action_Trooper/Meshes/Trooper_Hair/SK_M_Trooper_Beard_Thin.SK_M_Trooper_Beard_Thin" true)
                        (`PrimitiveComponent.SetMaterial` _hair_a__socketed_ 0 "/Game/Action_Trooper/Materials/Trooper_Hair/MI_Trooper_M_Hair_Brown.MI_Trooper_M_Hair_Brown")
                        (`PrimitiveComponent.SetMaterial` _hair_a__socketed_ 1 "/Game/Action_Trooper/Materials/Trooper_Heads_and_Bodies/M_Trooper_ShadowTrim.M_Trooper_ShadowTrim")
                        (`SkinnedMeshComponent.SetSkinnedAssetAndUpdate` _hair_b__socketed__2 "/Game/Action_Trooper/Meshes/Trooper_Hair/SK_M_Trooper_Beard_Thin.SK_M_Trooper_Beard_Thin" true)
                        (`PrimitiveComponent.SetMaterial` _hair_b__socketed__2 0 "/Game/Action_Trooper/Materials/Trooper_Hair/MI_Trooper_M_Hair_Dark_Brown.MI_Trooper_M_Hair_Dark_Brown")
                        (`PrimitiveComponent.SetMaterial` _hair_b__socketed__2 1 "/Game/Action_Trooper/Materials/Trooper_Heads_and_Bodies/M_Trooper_ShadowTrim.M_Trooper_ShadowTrim")
                        (`SkinnedMeshComponent.SetSkinnedAssetAndUpdate` _hair_c__socketed__3 null true)
                        (`PrimitiveComponent.SetMaterial` _hair_c__socketed__3 0 null)
                        (`PrimitiveComponent.SetMaterial` _hair_c__socketed__3 1 "/Game/Action_Trooper/Materials/Trooper_Heads_and_Bodies/M_Trooper_ShadowTrim.M_Trooper_ShadowTrim"))))
                  (:`then_1`
                    (`PrimitiveComponent.SetMaterial` _shoulders__skeletal__4 1 "/Game/Action_Trooper/Materials/Trooper_Armor/MI_Trooper_GloFX_Shoulders_Blueglo.MI_Trooper_GloFX_Shoulders_Blueglo")))))
            (:`then_1`
              (for _index_2 (range 3 5)
                (`PrimitiveComponent.SetMaterial` _mesh_8 _index_2 "/Game/Action_Trooper/Materials/Trooper_Heads_and_Bodies/MI_Trooper_M_Head_A_White.MI_Trooper_M_Head_A_White")))
            (:`then_2`
              (for _index_3 (range 2 3)
                (`PrimitiveComponent.SetMaterial` _mesh_8 _index_3 "/Game/Action_Trooper/Materials/Trooper_Heads_and_Bodies/M_Trooper_ShadowTrim.M_Trooper_ShadowTrim"))))
          (elif (== (`self.CharPresetIndex`) 1)
            ;[1 0.1745 0.7655] Set main Mesh component (full body or standalone head)
            (`SkeletalMeshComponent.SetAnimInstanceClass` _mesh_3 "/Game/Action_Trooper/Animations/Female/ThirdPerson_Female_AnimBP.ThirdPerson_Female_AnimBP_C")
            (`SkinnedMeshComponent.SetSkinnedAssetAndUpdate` _mesh_3 "/Game/Action_Trooper/Meshes/Trooper_Heads/SK_F_Trooper_Head_B_Black.SK_F_Trooper_Head_B_Black" false)
            ;[1 0.1745 0.7655] Set material(s) of body or head per ID
            (`|ExecutionSequence`
              (:`then_0`
                (for _index_4 (range 2)
                  (`PrimitiveComponent.SetMaterial` _mesh_4 _index_4 "/Game/Action_Trooper/Materials/Trooper_Heads_and_Bodies/MI_Trooper_F_Head_B_Black.MI_Trooper_F_Head_B_Black")))
              (:`then_1`
                (for _index_5 (range 3 5)
                  (`PrimitiveComponent.SetMaterial` _mesh_4 _index_5 "/Game/Action_Trooper/Materials/Trooper_Heads_and_Bodies/MI_Trooper_F_Head_B_Black.MI_Trooper_F_Head_B_Black")
                  ;[1 0.1745 0.7655] Set Upper armor and materials
                  (`SkeletalMeshComponent.SetAnimInstanceClass` _upper__skeletal__2 "/Game/Action_Trooper/Animations/Female/ThirdPerson_Female_AnimBP.ThirdPerson_Female_AnimBP_C")
                  (`SkinnedMeshComponent.SetSkinnedAssetAndUpdate` _upper__skeletal__2 "/Game/Action_Trooper/Meshes/Trooper_Armor_Modular/SK_F_Trooper_Upper.SK_F_Trooper_Upper" false)
                  (`|ExecutionSequence`
                    (:`then_0`
                      (`PrimitiveComponent.SetMaterial` _upper__skeletal_ 0 "/Game/Action_Trooper/Materials/Trooper_Armor/MI_Trooper_Upper_Tinted_PurpleLemon.MI_Trooper_Upper_Tinted_PurpleLemon"))
                    (:`then_1`
                      (`PrimitiveComponent.SetMaterial` _upper__skeletal_ 1 "/Game/Action_Trooper/Materials/Trooper_Armor/MI_Trooper_Shoulders_Tinted_PurpleLime.MI_Trooper_Shoulders_Tinted_PurpleLime")
                      ;[1 0.1745 0.7655] Set Lower armor compoment and material
                      (`SkeletalMeshComponent.SetAnimInstanceClass` _lower__skeketal_ "/Game/Action_Trooper/Animations/Female/ThirdPerson_Female_AnimBP.ThirdPerson_Female_AnimBP_C")
                      (`SkinnedMeshComponent.SetSkinnedAssetAndUpdate` _lower__skeketal_ "/Game/Action_Trooper/Meshes/Trooper_Armor_Modular/SK_F_Trooper_Lower.SK_F_Trooper_Lower" false)
                      (`PrimitiveComponent.SetMaterial` (`self.Lower (skeketal)`) 0 "/Game/Action_Trooper/Materials/Trooper_Armor/MI_Trooper_Lower_Tinted_PurpleLemon.MI_Trooper_Lower_Tinted_PurpleLemon")
                      ;[1 0.1745 0.7655] Set Shoulders and materials (left/right)
                      (`SkeletalMeshComponent.SetAnimInstanceClass` _shoulders__skeletal__2 "/Game/Action_Trooper/Animations/Female/ThirdPerson_Female_AnimBP.ThirdPerson_Female_AnimBP_C")
                      (`SkinnedMeshComponent.SetSkinnedAssetAndUpdate` _shoulders__skeletal__2 "/Game/Action_Trooper/Meshes/Trooper_Armor_Modular/SK_F_Trooper_Shoulders_C.SK_F_Trooper_Shoulders_C" false)
                      (`|ExecutionSequence`
                        (:`then_0`
                          (`PrimitiveComponent.SetMaterial` _shoulders__skeletal__2 0 "/Game/Action_Trooper/Materials/Trooper_Armor/MI_Trooper_Shoulders_Tinted_PurpleLime.MI_Trooper_Shoulders_Tinted_PurpleLime")
                          ;[1 0.1745 0.7655] Set Helmet
                          (`SkinnedMeshComponent.SetSkinnedAssetAndUpdate` _helmet__socketed__3 null true)
                          (`|ExecutionSequence`
                            (:`then_0`
                              (`PrimitiveComponent.SetMaterial` _helmet__socketed__3 2 null)
                              ;[1 0.1745 0.7655] Set Hair
                              (`SkinnedMeshComponent.SetSkinnedAssetAndUpdate` _hair_a__socketed__4 "/Game/Action_Trooper/Meshes/Trooper_Hair/SK_F_Trooper_Hair_Buns.SK_F_Trooper_Hair_Buns" true)
                              (`PrimitiveComponent.SetMaterial` _hair_a__socketed__4 0 "/Game/Action_Trooper/Materials/Trooper_Hair/MI_Trooper_M_Hair_Black_afro.MI_Trooper_M_Hair_Black_afro")
                              (`PrimitiveComponent.SetMaterial` _hair_a__socketed__4 1 "/Game/Action_Trooper/Materials/Trooper_Heads_and_Bodies/M_Trooper_ShadowTrim.M_Trooper_ShadowTrim")
                              (`SkinnedMeshComponent.SetSkinnedAssetAndUpdate` _hair_b__socketed__4 null true)
                              (`PrimitiveComponent.SetMaterial` _hair_b__socketed__4 0 null)
                              (`PrimitiveComponent.SetMaterial` _hair_b__socketed__4 1 "/Game/Action_Trooper/Materials/Trooper_Heads_and_Bodies/M_Trooper_ShadowTrim.M_Trooper_ShadowTrim")
                              (`SkinnedMeshComponent.SetSkinnedAssetAndUpdate` _hair_c__socketed__4 null true)
                              (`PrimitiveComponent.SetMaterial` _hair_c__socketed__4 0 "/Game/Action_Trooper/Materials/Trooper_Hair/MI_Trooper_M_Hair_Dark_Brown.MI_Trooper_M_Hair_Dark_Brown")
                              (`PrimitiveComponent.SetMaterial` _hair_c__socketed__4 1 "/Game/Action_Trooper/Materials/Trooper_Heads_and_Bodies/M_Trooper_ShadowTrim.M_Trooper_ShadowTrim"))))
                        (:`then_1`
                          (`PrimitiveComponent.SetMaterial` _shoulders__skeletal__2 1 "/Game/Action_Trooper/Materials/Trooper_Armor/MI_Trooper_Shoulders_Tinted_PurpleLime.MI_Trooper_Shoulders_Tinted_PurpleLime"))))
                    (:`then_2`
                      (`PrimitiveComponent.SetMaterial` _upper__skeletal_ 2 "/Game/Action_Trooper/Materials/Trooper_Armor/MI_Trooper_Shoulders_Tinted_PurpleLime.MI_Trooper_Shoulders_Tinted_PurpleLime")))))
              (:`then_2`
                (for _index_6 (range 2 3)
                  (`PrimitiveComponent.SetMaterial` _mesh_4 _index_6 "/Game/Action_Trooper/Materials/Trooper_Heads_and_Bodies/M_Trooper_ShadowTrim.M_Trooper_ShadowTrim"))))
            (elif (== (`self.CharPresetIndex`) 2)
              ;[1 0.1745 0.7655] Set main Mesh component (full body or standalone head)
              (`SkeletalMeshComponent.SetAnimInstanceClass` _mesh_6 "/Game/Action_Trooper/Animations/Female/ThirdPerson_Female_AnimBP.ThirdPerson_Female_AnimBP_C")
              (`SkinnedMeshComponent.SetSkinnedAssetAndUpdate` _mesh_6 "/Game/Action_Trooper/Meshes/Trooper_Heads/SK_F_Trooper_Head_A_Latina2.SK_F_Trooper_Head_A_Latina2" false)
              ;[1 0.1745 0.7655] Set material(s) of body or head per ID
              (`|ExecutionSequence`
                (:`then_0`
                  (for _index_7 (range 2)
                    (`PrimitiveComponent.SetMaterial` _mesh _index_7 "/Game/Action_Trooper/Materials/Trooper_Heads_and_Bodies/MI_Trooper_F_Head_A_Latina.MI_Trooper_F_Head_A_Latina")))
                (:`then_1`
                  (for _index_8 (range 3 5)
                    (`PrimitiveComponent.SetMaterial` _mesh _index_8 "/Game/Action_Trooper/Materials/Trooper_Heads_and_Bodies/MI_Trooper_F_Head_A_Latina.MI_Trooper_F_Head_A_Latina")
                    ;[1 0.1745 0.7655] Set Upper armor and material
                    (`SkeletalMeshComponent.SetAnimInstanceClass` _upper__skeletal__5 "/Game/Action_Trooper/Animations/Female/ThirdPerson_Female_AnimBP.ThirdPerson_Female_AnimBP_C")
                    (`SkinnedMeshComponent.SetSkinnedAssetAndUpdate` _upper__skeletal__5 "/Game/Action_Trooper/Meshes/Trooper_Armor_Modular/SK_F_Trooper_Upper.SK_F_Trooper_Upper" false)
                    (`PrimitiveComponent.SetMaterial` _upper__skeletal__5 0 "/Game/Action_Trooper/Materials/Trooper_Armor/MI_Trooper_Upper_Tinted_White.MI_Trooper_Upper_Tinted_White")
                    ;[1 0.1745 0.7655] Set Lower compoment and material
                    (`SkeletalMeshComponent.SetAnimInstanceClass` _lower__skeketal__2 "/Game/Action_Trooper/Animations/Female/ThirdPerson_Female_AnimBP.ThirdPerson_Female_AnimBP_C")
                    (`SkinnedMeshComponent.SetSkinnedAssetAndUpdate` _lower__skeketal__2 "/Game/Action_Trooper/Meshes/Trooper_Armor_Modular/SK_F_Trooper_Lower.SK_F_Trooper_Lower" false)
                    (`PrimitiveComponent.SetMaterial` _lower__skeketal__2 0 "/Game/Action_Trooper/Materials/Trooper_Armor/MI_Trooper_NoTint_Lower_WhitePlastic.MI_Trooper_NoTint_Lower_Whiteplastic")
                    ;[1 0.1745 0.7655] Set Shoulders and materials (left/right)
                    (`SkeletalMeshComponent.SetAnimInstanceClass` _shoulders__skeletal_ "/Game/Action_Trooper/Animations/Female/ThirdPerson_Female_AnimBP.ThirdPerson_Female_AnimBP_C")
                    (`SkinnedMeshComponent.SetSkinnedAssetAndUpdate` _shoulders__skeletal_ "/Game/Action_Trooper/Meshes/Trooper_Armor_Modular/SK_F_Trooper_Shoulders_B.SK_F_Trooper_Shoulders_B" false)
                    (`|ExecutionSequence`
                      (:`then_0`
                        (`PrimitiveComponent.SetMaterial` _shoulders__skeletal_ 0 "/Game/Action_Trooper/Materials/Trooper_Armor/MI_Trooper_Shoulders_NoTint_Milit.MI_Trooper_Shoulders_NoTint_Milit")
                        ;[1 0.1745 0.7655] Set Helmet
                        (`SkinnedMeshComponent.SetSkinnedAssetAndUpdate` _helmet__socketed_ null true)
                        (`|ExecutionSequence`
                          (:`then_0`
                            (`PrimitiveComponent.SetMaterial` _helmet__socketed_ 0 null)
                            ;[1 0.1745 0.7655] Set Hair
                            (`SkinnedMeshComponent.SetSkinnedAssetAndUpdate` _hair_a__socketed__3 "/Game/Action_Trooper/Meshes/Trooper_Hair/SK_F_Trooper_Hair_long_with_bandana_strap.SK_F_Trooper_Hair_Long_with_bandana_strap" true)
                            (`PrimitiveComponent.SetMaterial` _hair_a__socketed__3 0 "/Game/Action_Trooper/Materials/Trooper_Hair/MI_Trooper_M_Hair_Dark_Brown.MI_Trooper_M_Hair_Dark_Brown")
                            (`PrimitiveComponent.SetMaterial` _hair_a__socketed__3 1 "/Game/Action_Trooper/Materials/Trooper_Heads_and_Bodies/M_Trooper_ShadowTrim.M_Trooper_ShadowTrim")
                            (`SkinnedMeshComponent.SetSkinnedAssetAndUpdate` _hair_b__socketed__3 "/Game/Action_Trooper/Meshes/Trooper_Hair/SK_F_Trooper_Hair_Bandana_knot.SK_F_Trooper_Hair_Bandana_knot" true)
                            (`PrimitiveComponent.SetMaterial` _hair_b__socketed__3 0 "/Game/Action_Trooper/Materials/Trooper_Hair/MI_Trooper_M_Hair_Brown.MI_Trooper_M_Hair_Brown")
                            (`PrimitiveComponent.SetMaterial` _hair_b__socketed__3 1 "/Game/Action_Trooper/Materials/Trooper_Heads_and_Bodies/M_Trooper_ShadowTrim.M_Trooper_ShadowTrim")
                            (`SkinnedMeshComponent.SetSkinnedAssetAndUpdate` _hair_c__socketed_ null true)
                            (`PrimitiveComponent.SetMaterial` _hair_c__socketed_ 0 "/Game/Action_Trooper/Materials/Trooper_Hair/MI_Trooper_M_Hair_Black.MI_Trooper_M_Hair_Black")
                            (`PrimitiveComponent.SetMaterial` _hair_c__socketed_ 1 "/Game/Action_Trooper/Materials/Trooper_Heads_and_Bodies/M_Trooper_ShadowTrim.M_Trooper_ShadowTrim"))))
                      (:`then_1`
                        (`PrimitiveComponent.SetMaterial` _shoulders__skeletal_ 1 "/Game/Action_Trooper/Materials/Trooper_Armor/MI_Trooper_Shoulders_NoTint_Milit.MI_Trooper_Shoulders_NoTint_Milit")))))
                (:`then_2`
                  (for _index_9 (range 2 3)
                    (`PrimitiveComponent.SetMaterial` _mesh _index_9 "/Game/Action_Trooper/Materials/Trooper_Heads_and_Bodies/M_Trooper_ShadowTrim.M_Trooper_ShadowTrim"))))
              (elif (== (`self.CharPresetIndex`) 3)
                ;[0.02924 0.4632 1] Set main Mesh component (full body or standalone head)
                (`SkeletalMeshComponent.SetAnimInstanceClass` _mesh_7 "/Game/Action_Trooper/Animations/Male/ThirdPerson_Male_AnimBP.ThirdPerson_Male_AnimBP_C")
                (`SkinnedMeshComponent.SetSkinnedAssetAndUpdate` _mesh_7 "/Game/Action_Trooper/Meshes/Trooper_Heads/SK_M_Trooper_Head_B_Latino.SK_M_Trooper_Head_B_Latino" false)
                ;[0.02745 0.4627 1] Set material(s) of body or head per ID
                (`|ExecutionSequence`
                  (:`then_0`
                    (for _index_10 (range 2)
                      (`PrimitiveComponent.SetMaterial` _mesh_9 _index_10 "/Game/Action_Trooper/Materials/Trooper_Heads_and_Bodies/MI_Trooper_M_Head_B_Latino2.MI_Trooper_M_Head_B_Latino2")
                      ;[0.02745 0.4627 1] Set Upper armor component (case of chest and shoulders as single mesh)
                      (`SkeletalMeshComponent.SetAnimInstanceClass` _upper__skeletal__3 "/Game/Action_Trooper/Animations/Male/ThirdPerson_Male_AnimBP.ThirdPerson_Male_AnimBP_C")
                      (`SkinnedMeshComponent.SetSkinnedAssetAndUpdate` _upper__skeletal__3 "/Game/Action_Trooper/Meshes/Trooper_Armor_Modular/SK_M_Trooper_Upper.SK_M_Trooper_Upper" false)
                      (`PrimitiveComponent.SetMaterial` (`self.Upper (skeletal)`) 0 "/Game/Action_Trooper/Materials/Trooper_Armor/MI_Trooper_Upper_NoTint_Aquablue.MI_Trooper_Upper_NoTint_Aquablue")
                      ;[0.02924 0.4632 1] Set Lower armor material
                      (`SkeletalMeshComponent.SetAnimInstanceClass` _lower__skeketal__5 "/Game/Action_Trooper/Animations/Male/ThirdPerson_Male_AnimBP.ThirdPerson_Male_AnimBP_C")
                      (`SkinnedMeshComponent.SetSkinnedAssetAndUpdate` _lower__skeketal__5 "/Game/Action_Trooper/Meshes/Trooper_Armor_Modular/SK_M_Trooper_Lower.SK_M_Trooper_Lower" false)
                      (`PrimitiveComponent.SetMaterial` (`self.Lower (skeketal)`) 0 "/Game/Action_Trooper/Materials/Trooper_Armor/MI_Trooper_Lower_NoTint_Aquablue.MI_Trooper_Lower_NoTint_Aquablue")
                      ;[0.02745 0.4627 1] Set Shoulders and materials (left/right)
                      (`SkeletalMeshComponent.SetAnimInstanceClass` _shoulders__skeletal__5 "/Game/Action_Trooper/Animations/Male/ThirdPerson_Male_AnimBP.ThirdPerson_Male_AnimBP_C")
                      (`SkinnedMeshComponent.SetSkinnedAssetAndUpdate` _shoulders__skeletal__5 "/Game/Action_Trooper/Meshes/Trooper_Armor_Modular/SK_M_Trooper_Shoulders_A.SK_M_Trooper_Shoulders_A" false)
                      (`|ExecutionSequence`
                        (:`then_0`
                          (`PrimitiveComponent.SetMaterial` _shoulders__skeletal__5 0 "/Game/Action_Trooper/Materials/Trooper_Armor/MI_Trooper_GloFX_Shoulders_Greenglo.MI_Trooper_GloFX_Shoulders_Greenglo")
                          ;[0.02924 0.4632 1] Set Helmet
                          (`SkinnedMeshComponent.SetSkinnedAssetAndUpdate` _helmet__socketed__5 "/Game/Action_Trooper/Meshes/Trooper_Helmets/SK_M_Trooper_Helmet_F.SK_M_Trooper_Helmet_F" true)
                          (`|ExecutionSequence`
                            (:`then_0`
                              (`PrimitiveComponent.SetMaterial` _helmet__socketed__5 2 "/Game/Action_Trooper/Materials/Trooper_Armor/MI_Trooper_Helmet_NoTint_Blue.MI_Trooper_Helmet_NoTint_Blue")
                              ;[0.02924 0.4632 1] Set hair and beard
                              (`SkinnedMeshComponent.SetSkinnedAssetAndUpdate` _hair_a__socketed__5 "/Game/Action_Trooper/Meshes/Trooper_Hair/SK_M_Trooper_Hair_Thin_with_sides.SK_M_Trooper_Hair_Thin_with_sides" true)
                              (`PrimitiveComponent.SetMaterial` _hair_a__socketed__5 0 "/Game/Action_Trooper/Materials/Trooper_Hair/MI_Trooper_M_Hair_Black.MI_Trooper_M_Hair_Black")
                              (`PrimitiveComponent.SetMaterial` _hair_a__socketed__5 1 "/Game/Action_Trooper/Materials/Trooper_Heads_and_Bodies/M_Trooper_ShadowTrim.M_Trooper_ShadowTrim")
                              (`SkinnedMeshComponent.SetSkinnedAssetAndUpdate` _hair_b__socketed__5 "/Game/Action_Trooper/Meshes/Trooper_Hair/SK_M_Trooper_Beard_Thin.SK_M_Trooper_Beard_Thin" true)
                              (`PrimitiveComponent.SetMaterial` _hair_b__socketed__5 0 "/Game/Action_Trooper/Materials/Trooper_Hair/MI_Trooper_M_Hair_Black.MI_Trooper_M_Hair_Black")
                              (`PrimitiveComponent.SetMaterial` _hair_b__socketed__5 1 "/Game/Action_Trooper/Materials/Trooper_Heads_and_Bodies/M_Trooper_ShadowTrim.M_Trooper_ShadowTrim")
                              (`SkinnedMeshComponent.SetSkinnedAssetAndUpdate` _hair_c__socketed__5 null true)
                              (`PrimitiveComponent.SetMaterial` _hair_c__socketed__5 0 "/Game/Action_Trooper/Materials/Trooper_Hair/MI_Trooper_M_Hair_Black.MI_Trooper_M_Hair_Black")
                              (`PrimitiveComponent.SetMaterial` _hair_c__socketed__5 1 "/Game/Action_Trooper/Materials/Trooper_Heads_and_Bodies/M_Trooper_ShadowTrim.M_Trooper_ShadowTrim"))))
                        (:`then_1`
                          (`PrimitiveComponent.SetMaterial` _shoulders__skeletal__5 1 "/Game/Action_Trooper/Materials/Trooper_Armor/MI_Trooper_GloFX_Shoulders_Greenglo.MI_Trooper_GloFX_Shoulders_Greenglo")))))
                  (:`then_1`
                    (for _index_11 (range 3 5)
                      (`PrimitiveComponent.SetMaterial` _mesh_9 _index_11 "/Game/Action_Trooper/Materials/Trooper_Heads_and_Bodies/MI_Trooper_M_Head_B_Latino2.MI_Trooper_M_Head_B_Latino2")))
                  (:`then_2`
                    (for _index_12 (range 2 3)
                      (`PrimitiveComponent.SetMaterial` _mesh_9 _index_12 "/Game/Action_Trooper/Materials/Trooper_Heads_and_Bodies/M_Trooper_ShadowTrim.M_Trooper_ShadowTrim"))))
                (elif (== (`self.CharPresetIndex`) 4)
                  ;[0.02924 0.4632 1] Set main Mesh component (full body or standalone head)
                  (`SkeletalMeshComponent.SetAnimInstanceClass` _mesh_10 "/Game/Action_Trooper/Animations/Male/ThirdPerson_Male_AnimBP.ThirdPerson_Male_AnimBP_C")
                  (`SkinnedMeshComponent.SetSkinnedAssetAndUpdate` _mesh_10 "/Game/Action_Trooper/Meshes/BodyForms/SK_Male_Form_Head.SK_Male_Form_Head" false)
                  ;[0.02745 0.4627 1] Set material(s) of body or head per ID
                  (`PrimitiveComponent.SetMaterial` (`self.Mesh`) 0 null)
                  ;[0.02745 0.4627 1] Set Upper armor component (case of chest and shoulders as single mesh)
                  (`SkeletalMeshComponent.SetAnimInstanceClass` _upper__skeletal__7 "/Game/Action_Trooper/Animations/Male/ThirdPerson_Male_AnimBP.ThirdPerson_Male_AnimBP_C")
                  (`SkinnedMeshComponent.SetSkinnedAssetAndUpdate` _upper__skeletal__7 "/Game/Action_Trooper/Meshes/BodyForms/SK_Male_Form_Upper.SK_Male_Form_Upper" false)
                  (`PrimitiveComponent.SetMaterial` (`self.Upper (skeletal)`) 0 null)
                  ;[0.02924 0.4632 1] Set Lower armor material
                  (`SkeletalMeshComponent.SetAnimInstanceClass` _lower__skeketal__6 "/Game/Action_Trooper/Animations/Male/ThirdPerson_Male_AnimBP.ThirdPerson_Male_AnimBP_C")
                  (`SkinnedMeshComponent.SetSkinnedAssetAndUpdate` _lower__skeketal__6 "/Game/Action_Trooper/Meshes/BodyForms/SK_Male_Form_Lower.SK_Male_Form_Lower" false)
                  (`PrimitiveComponent.SetMaterial` (`self.Lower (skeketal)`) 0 null)
                  ;[0.02745 0.4627 1] Set Shoulders and materials (left/right)
                  (`SkeletalMeshComponent.SetAnimInstanceClass` _shoulders__skeletal__6 "/Game/Action_Trooper/Animations/Male/ThirdPerson_Male_AnimBP.ThirdPerson_Male_AnimBP_C")
                  (`SkinnedMeshComponent.SetSkinnedAssetAndUpdate` _shoulders__skeletal__6 null false)
                  (`PrimitiveComponent.SetMaterial` _shoulders__skeletal__6 0 "/Game/Action_Trooper/Materials/Trooper_Armor/MI_Trooper_GloFX_Shoulders_Greenglo.MI_Trooper_GloFX_Shoulders_Greenglo")
                  ;[0.02924 0.4632 1] Set Helmet
                  (`SkinnedMeshComponent.SetSkinnedAssetAndUpdate` _helmet__socketed__6 null true)
                  (`PrimitiveComponent.SetMaterial` _helmet__socketed__6 2 "/Game/Action_Trooper/Materials/Trooper_Armor/MI_Trooper_Helmet_NoTint_Blue.MI_Trooper_Helmet_NoTint_Blue")
                  ;[0.02924 0.4632 1] Set hair and beard
                  (`SkinnedMeshComponent.SetSkinnedAssetAndUpdate` _hair_a__socketed__6 null true)
                  (`PrimitiveComponent.SetMaterial` _hair_a__socketed__6 0 null)
                  (`PrimitiveComponent.SetMaterial` _hair_a__socketed__6 1 null)
                  (`SkinnedMeshComponent.SetSkinnedAssetAndUpdate` _hair_b__socketed__6 null true)
                  (`PrimitiveComponent.SetMaterial` _hair_b__socketed__6 0 null)
                  (`PrimitiveComponent.SetMaterial` _hair_b__socketed__6 1 null)
                  (`SkinnedMeshComponent.SetSkinnedAssetAndUpdate` _hair_c__socketed__6 null true)
                  (`PrimitiveComponent.SetMaterial` _hair_c__socketed__6 0 null)
                  (`PrimitiveComponent.SetMaterial` _hair_c__socketed__6 1 null)
                  (elif (== (`self.CharPresetIndex`) 5)
                    ;[1 0.1745 0.7655] Set main Mesh component (full body or standalone head)
                    (`SkeletalMeshComponent.SetAnimInstanceClass` _mesh_5 "/Game/Action_Trooper/Animations/Female/ThirdPerson_Female_AnimBP.ThirdPerson_Female_AnimBP_C")
                    (`SkinnedMeshComponent.SetSkinnedAssetAndUpdate` _mesh_5 "/Game/Action_Trooper/Meshes/BodyForms/SK_Female_Form_Head.SK_Female_Form_Head" false)
                    ;[1 0.1745 0.7655] Set material(s) of body or head per ID
                    (`PrimitiveComponent.SetMaterial` (`self.Mesh`) 0 null)
                    ;[1 0.1745 0.7655] Set Upper armor component (case of chest and shoulders as single mesh)
                    (`SkeletalMeshComponent.SetAnimInstanceClass` _upper__skeletal__4 "/Game/Action_Trooper/Animations/Female/ThirdPerson_Female_AnimBP.ThirdPerson_Female_AnimBP_C")
                    (`SkinnedMeshComponent.SetSkinnedAssetAndUpdate` _upper__skeletal__4 "/Game/Action_Trooper/Meshes/BodyForms/SK_Female_Form_Upper.SK_Female_Form_Upper" false)
                    (`PrimitiveComponent.SetMaterial` (`self.Upper (skeletal)`) 0 null)
                    ;[1 0.1745 0.7655] Set Lower armor material
                    (`SkeletalMeshComponent.SetAnimInstanceClass` _lower__skeketal__3 "/Game/Action_Trooper/Animations/Female/ThirdPerson_Female_AnimBP.ThirdPerson_Female_AnimBP_C")
                    (`SkinnedMeshComponent.SetSkinnedAssetAndUpdate` _lower__skeketal__3 "/Game/Action_Trooper/Meshes/BodyForms/SK_Female_Form_Lower.SK_Female_Form_Lower" false)
                    (`PrimitiveComponent.SetMaterial` (`self.Lower (skeketal)`) 0 null)
                    ;[1 0.1745 0.7655] Set Shoulders and materials (left/right)
                    (`SkeletalMeshComponent.SetAnimInstanceClass` _shoulders__skeletal__3 "/Game/Action_Trooper/Animations/Female/ThirdPerson_Female_AnimBP.ThirdPerson_Female_AnimBP_C")
                    (`SkinnedMeshComponent.SetSkinnedAssetAndUpdate` _shoulders__skeletal__3 null false)
                    (`PrimitiveComponent.SetMaterial` _shoulders__skeletal__3 0 "/Game/Action_Trooper/Materials/Trooper_Armor/MI_Trooper_GloFX_Shoulders_Greenglo.MI_Trooper_GloFX_Shoulders_Greenglo")
                    ;[1 0.1745 0.7655] Set Helmet
                    (`SkinnedMeshComponent.SetSkinnedAssetAndUpdate` _helmet__socketed__2 null true)
                    (`PrimitiveComponent.SetMaterial` _helmet__socketed__2 2 "/Game/Action_Trooper/Materials/Trooper_Armor/MI_Trooper_Helmet_NoTint_Blue.MI_Trooper_Helmet_NoTint_Blue")
                    ;[1 0.1745 0.7655] Set hair and beard
                    (`SkinnedMeshComponent.SetSkinnedAssetAndUpdate` _hair_a__socketed__2 null true)
                    (`PrimitiveComponent.SetMaterial` _hair_a__socketed__2 0 null)
                    (`PrimitiveComponent.SetMaterial` _hair_a__socketed__2 1 null)
                    (`SkinnedMeshComponent.SetSkinnedAssetAndUpdate` _hair_b__socketed_ null true)
                    (`PrimitiveComponent.SetMaterial` _hair_b__socketed_ 0 null)
                    (`PrimitiveComponent.SetMaterial` _hair_b__socketed_ 1 null)
                    (`SkinnedMeshComponent.SetSkinnedAssetAndUpdate` _hair_c__socketed__2 null true)
                    (`PrimitiveComponent.SetMaterial` _hair_c__socketed__2 0 null)
                    (`PrimitiveComponent.SetMaterial` _hair_c__socketed__2 1 null)
                    (elif (== (`self.CharPresetIndex`) 6)
                      _
                      (elif (== (`self.CharPresetIndex`) 7)
                        _))))))))))))

(event `Key|E`
  (params (Key :type "Key Structure"))
  (:`Pressed`
    (goto _label)))

(fn `IncomingDamage`
  (params (NewParam :type "Float (double-precision)"))
  (bind _health (`self.Health`))
  (set `self.Health` (- _health NewParam))
  (if (<= _health 0.0)
    (`self.K2_DestroyActor`)))

(fn `UserConstructionScript`
  (`SkinnedMeshComponent.SetLeaderPoseComponent` (`self.Lower (skeketal)`) (`self.Mesh`) true)
  (`SkinnedMeshComponent.SetLeaderPoseComponent` (`self.Upper (skeletal)`) (`self.Mesh`) true)
  (`SkinnedMeshComponent.SetLeaderPoseComponent` (`self.Shoulders (skeletal)`) (`self.Mesh`) true))